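; BP_MainGame is a manager Blueprint for a 2D Snake game that spawns snake body parts and food.
; SpawnFood picks a random X/Z point inside the XMax/ZMax bounds, snaps it to a 100-unit grid and stores the food actor.
; SpawnNewSnakePart only spawns the body actor at a given location.
; Its head/body flipbook, IsHead, random rotation and SnakePartsArray setup are disconnected and never run.
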(event `Spawn New Snake Part`
  (params (`Spawn Location` :type "Vector Structure") (`Is Head` :type Boolean))
  ;[1 1 1] Spawn New Snake Part
  (bind _returnvalue (`|SpawnActorFromClass` "/Game/Blueprints/BP_SnakeBodyPart.BP_SnakeBodyPart_C" (`KismetMathLibrary.MakeTransform` `Spawn Location`) "AlwaysSpawn" "OverrideRootScale" null null)))

(event `Spawn Food`
  (bind _returnvalue (- (`self.Z_Max`) 100.0))
  (bind _returnvalue_2 (- (`self.X_Max`) 100.0))
  ;[1 1 1] Spawn Food
  (bind _returnvalue_3 (`|SpawnActorFromClass` "/Game/Blueprints/BP_Food.BP_Food_C" (`KismetMathLibrary.MakeTransform` (`KismetMathLibrary.MakeVector` (* (`.ReturnValue` (`KismetMathLibrary.FMod` (`KismetMathLibrary.RandomFloatInRange` (* _returnvalue_2 -1.0) _returnvalue_2) 100.0)) 100.0) -0.1 (* (`.ReturnValue` (`KismetMathLibrary.FMod` (`KismetMathLibrary.RandomFloatInRange` (* _returnvalue -1.0) _returnvalue) 100.0)) 100.0))) "AlwaysSpawn" "OverrideRootScale" null null))
  (set `self.Food Actor REF` _returnvalue_3))

(fn `UserConstructionScript`)