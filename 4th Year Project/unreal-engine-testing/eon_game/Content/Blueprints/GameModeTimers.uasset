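; GameModeTimers is a Blueprint that runs a minutes-and-seconds game countdown, printing "Game Over" and pausing the game at zero.
; Tick feeds a one-second Delay that gates each decrement, borrowing from Minutes when Seconds drops below zero.
; An unconnected count-up variant sits in the Event Graph and never runs.
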(event `self.ReceiveTick`
  (params (DeltaSeconds :type "Float (single-precision)"))
  ;[1 1 1] Game Countdown Timer
  ;;[1 1 1] Decrements Game Time per second
  (`KismetSystemLibrary.Delay` 1.0)
  (set `self.Seconds` (- (`self.Seconds`) 1))
  (if (< (`self.Seconds`) 0)
    (set `self.Minutes` (- (`self.Minutes`) 1))
    (set `self.Seconds` 59)
    (else
      ;;[1 1 1] Checks if seconds and minutes both == 0
      (if (== (`self.Seconds`) 0)
        (if (== (`self.Minutes`) 0)
          (`KismetSystemLibrary.PrintString` "Game Over")
          (`GameplayStatics.SetGamePaused` true))))))

(fn `UserConstructionScript`)