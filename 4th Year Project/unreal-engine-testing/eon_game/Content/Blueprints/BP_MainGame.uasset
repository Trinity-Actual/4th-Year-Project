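; BP_MainGame is a game-flow actor that creates the HUD, watches the game timer and handles level restart.
; Each tick it reads and prints GameModeTimers seconds, setting GameOver and firing the HUD's game-over event when minutes and seconds reach zero.
; After game over, Tick feeds a Gate that the R key opens, then a DoOnce removes the HUD and reloads the current level.
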(event `self.ReceiveBeginPlay`
  (bind _returnvalue (`|CreateWidget` "/Game/Blueprints/BP_UI_HUD.BP_UI_HUD_C"))
  (bind _output_get (set `self.HUD_REF` _returnvalue))
  (`UserWidget.AddToViewport` _output_get 0))

(event `self.ReceiveTick`
  (params (DeltaSeconds :type "Float (single-precision)"))
  ;[1 1 1] Easy Example to Reference Variables from Gamemode Blueprint, can also use this as a method of obtaining Game time number
  (if (`self.Game Over`)
    (`/Engine/EditorBlueprintResources/StandardMacros.Gate` true :!label _label
      (:`Exit`
        (`/Engine/EditorBlueprintResources/StandardMacros.DoOnce` false
          (:`Completed`
            (`Widget.RemoveFromParent` (`self.HUD_REF`))
            (bind _returnvalue (`GameplayStatics.GetCurrentLevelName` true))
            (`GameplayStatics.OpenLevel` (`KismetStringLibrary.Conv_StringToName` _returnvalue))))))
    (else
      (bind _asgame_mode_timers (cast `/Game/Blueprints/GameModeTimers` (`GameplayStatics.GetGameMode`)))
      (bind _seconds (`/Game/Blueprints/GameModeTimers.Seconds` _asgame_mode_timers))
      (`KismetSystemLibrary.PrintString` (`KismetStringLibrary.Conv_IntToString` _seconds))
      (if (== _seconds 0)
        (if (== (`/Game/Blueprints/GameModeTimers.Minutes` _asgame_mode_timers) 0)
          (set `self.Game Over` true)
          (`/Game/Blueprints/BP_UI_HUD.Game Over Event` (`self.HUD_REF`)))))))

(event `Key|R`
  (params (Key :type "Key Structure"))
  ;[1 1 1] Easy Example to Reference Variables from Gamemode Blueprint, can also use this as a method of obtaining Game time number
  (:`Pressed`
    (goto _label :!via `Open`)))

(fn `UserConstructionScript`)